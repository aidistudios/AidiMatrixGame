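; Endless-runner tunnel segment with a rotating holed wall that scores the player for passing and damages them on collision.
; BeginPlay randomly spawns a health pack or enemy ahead, with a chance of an extra enemy.
; Passing the trigger or hitting the wall, which also shakes the camera, makes TunnelSpawner add a segment and destroys this one.
; RandomizeWall picks a hole mesh and roll, but is not called here.
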(event OnComponentBeginOverlap(TriggerZone)
  (params (OverlappedComponent :type Primitive%20Component%20Object%20Reference) (OtherActor :type Actor%20Object%20Reference) (OtherComp :type Primitive%20Component%20Object%20Reference) (OtherBodyIndex :type Integer) (bFromSweep :type Boolean) (SweepResult :type Hit%20Result%20Structure%20%28by%20ref%29))
  (bind _asbp_player (Utilities|Casting|CastToBP_Player OtherActor))
  (Variables|/Game/InfiniteMatrix/Blueprints/BP_Player.BP_Player_C|SetScore _asbp_player (+ (Variables|/Game/InfiniteMatrix/Blueprints/BP_Player.BP_Player_C|GetScore _asbp_player) 1))
  (Default|UpdateScore _asbp_player)
  (Default|SpawnTunnelatSpawnPoint (Variables|Default|GetTunnelSpawner))
  (Actor|DestroyActor))

(event OnComponentBeginOverlap(WallMesh)
  (params (OverlappedComponent :type Primitive%20Component%20Object%20Reference) (OtherActor :type Actor%20Object%20Reference) (OtherComp :type Primitive%20Component%20Object%20Reference) (OtherBodyIndex :type Integer) (bFromSweep :type Boolean) (SweepResult :type Hit%20Result%20Structure%20%28by%20ref%29))
  (bind _asbp_player (Utilities|Casting|CastToBP_Player OtherActor))
  (Components|DestroyComponent (Variables|Default|GetTriggerZone))
  (Default|UpdateHealthBar _asbp_player (Variables|Default|GetCollisionDamage))
  (Camera|PlayWorldCameraShake "/Game/InfiniteMatrix/Blueprints/BP_CameraShake.BP_CameraShake_C" (Transformation|GetActorLocation _asbp_player) 0.0 5e+02)
  (Default|SpawnTunnelatSpawnPoint (Variables|Default|GetTunnelSpawner))
  (Actor|DestroyActor))

(event EventBeginPlay
  (Utilities|FlowControl|Sequence
    (:then_0
      (if (>= (Math|Random|RandomFloat) 0.6)
        (CallFunction|SpawnHealthPack)
        (else
          (CallFunction|SpawnEnemy))))
    (:then_1
      (if (>= (Math|Random|RandomFloatinRange 0.0 1.0) 0.5)
        (CallFunction|SpawnEnemy)))))

(event EventTick
  (params (DeltaSeconds :type Float%20%28single-precision%29))
  (Transformation|AddLocalRotation (Variables|Default|GetWallMesh) (Math|Rotator|MakeRotator (* DeltaSeconds (Variables|Default|GetRotateSpeed)) 0.0 0.0) false false))

(fn ConstructionScript)

(fn RandomizeWall
  (Components|StaticMesh|SetStaticMesh (Variables|Default|GetWallMesh) (Utilities|Select :Index (Math|Random|RandomIntegerinRange 0 3) :Option%200 "/Game/InfiniteMatrix/Meshes/SM_Hole_01.SM_Hole_01" :Option%201 "/Game/InfiniteMatrix/Meshes/SM_Hole_02.SM_Hole_02" :Option%202 "/Game/InfiniteMatrix/Meshes/SM_Hole_03.SM_Hole_03" :Option%203 "/Game/InfiniteMatrix/Meshes/SM_Hole_04.SM_Hole_04"))
  (Transformation|AddLocalRotation (Variables|Default|GetWallMesh) (Math|Rotator|MakeRotator (Math|Random|RandomFloatinRange 0.0 3.6e+02) 0.0 0.0) false false))

(fn SpawnHealthPack
  (bind _origin (Variables|Default|GetOrigin))
  (bind _returnvalue (Transformation|GetWorldLocation _origin))
  (Game|SpawnActorfromClass "/Game/InfiniteMatrix/Blueprints/BP_HealthPack.BP_HealthPack_C" (Math|Conversions|ToTransform(Vector) (Math|Vector|MakeVector (+ (.x _returnvalue) (Math|Random|RandomFloatinRange 5e+02 2e+03)) (+ (.y _returnvalue) (Math|Random|RandomFloatinRange -3e+02 3e+02)) (+ (.z _returnvalue) (Math|Random|RandomFloatinRange -3e+02 3e+02)))) "Undefined" 0 0))

(fn SpawnEnemy
  (bind _returnvalue (Math|Random|RandomFloatinRange 0.8 1.5))
  (bind _origin (Variables|Default|GetOrigin))
  (bind _returnvalue_2 (Transformation|GetWorldLocation _origin))
  (bind _returnvalue_3 (* _returnvalue 6.0))
  (Game|SpawnActorfromClass "/Game/InfiniteMatrix/Blueprints/BP_Enemy.BP_Enemy_C" (Math|Transform|MakeTransform (Math|Vector|MakeVector (+ (.x _returnvalue_2) (Math|Random|RandomFloatinRange 5e+02 2e+03)) (+ (.y _returnvalue_2) (Math|Random|RandomFloatinRange -3e+02 3e+02)) (+ (.z _returnvalue_2) (Math|Random|RandomFloatinRange -3e+02 3e+02))) "0, 0, 0" (Math|Vector|MakeVector _returnvalue_3 _returnvalue_3 _returnvalue_3)) "Undefined" 0 0))
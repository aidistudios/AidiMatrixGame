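; BP_Projectile is a projectile that destroys enemies and awards score to the player.
; Tick moves it along world X at ForwardSpeed with a swept offset, and it destroys itself after the DestroyAfter delay.
; On sphere trigger overlap, a BP_Enemy adds its ScoreIncrement to the Player's score, then both actors are destroyed.
; Other overlaps destroy the projectile, except BP_Player and box components, which it ignores.
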(event OnComponentBeginOverlap(SphereTrigger)
  (params (OverlappedComponent :type Primitive%20Component%20Object%20Reference) (OtherActor :type Actor%20Object%20Reference) (OtherComp :type Primitive%20Component%20Object%20Reference) (OtherBodyIndex :type Integer) (bFromSweep :type Boolean) (SweepResult :type Hit%20Result%20Structure%20%28by%20ref%29))
  (bind _player (Variables|Default|GetPlayer))
  (bind _asbp_enemy (Utilities|Casting|CastToBP_Enemy OtherActor)
    (:then
      (Variables|/Game/InfiniteMatrix/Blueprints/BP_Player.BP_Player_C|SetScore _player (+ (Variables|/Game/InfiniteMatrix/Blueprints/BP_Player.BP_Player_C|GetScore _player) (Variables|/Game/InfiniteMatrix/Blueprints/BP_Enemy.BP_Enemy_C|GetScoreIncrement _asbp_enemy)))
      (Default|UpdateScore _player)
      (Actor|DestroyActor _asbp_enemy)
      (Actor|DestroyActor))
    (:CastFailed
      (Utilities|Casting|CastToBP_Player OtherActor
        (:CastFailed
          (Utilities|Casting|CastToBoxComponent OtherComp
            (:CastFailed
              (Actor|DestroyActor))))))))

(event EventBeginPlay
  (Utilities|FlowControl|Delay (Variables|Default|GetDestroyAfter))
  (Actor|DestroyActor))

(event Collision|EventActorBeginOverlap
  (params (OtherActor :type Actor%20Object%20Reference)))

(event EventTick
  (params (DeltaSeconds :type Float%20%28single-precision%29))
  (Transformation|AddActorWorldOffset (Math|Vector|MakeVector (* DeltaSeconds (Variables|Default|GetforwardSpeed)) 0.0 0.0) true))

(fn ConstructionScript)